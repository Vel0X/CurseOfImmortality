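; Custom game mode that owns the upgrade menu and death screen widgets and shows them on request.
; BeginPlay creates both widgets for the first player controller and stores them.
; Two custom events add the matching widget to the viewport and switch to Game and UI input, focusing a button on it.
; A DoOnce with no reset keeps the death screen from being shown more than once.
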(event `self.ReceiveBeginPlay`
  (bind _returnvalue (`GameplayStatics.GetPlayerController` 0))
  (bind _returnvalue_2 (`|CreateWidget` "/Game/UI/UpgradeMenu.UpgradeMenu_C" _returnvalue))
  (set `self.UpradeMenu` _returnvalue_2)
  (bind _returnvalue_3 (`|CreateWidget` "/Game/UI/DeathScreen.DeathScreen_C" _returnvalue))
  (set `self.DeathScreen` _returnvalue_3))

(event `self.ShowUpgradeMenu`
  (`UserWidget.AddToViewport` (`self.UpradeMenu`) 0)
  (`WidgetBlueprintLibrary.SetInputMode_GameAndUIEx` (`GameplayStatics.GetPlayerController` 0) (`/Game/UI/UpgradeMenu.Button_Middle` (stale `self.ReceiveBeginPlay` _returnvalue_2)) "DoNotLock" false))

(event `self.ShowDeathScreen`
  (`/Engine/EditorBlueprintResources/StandardMacros.DoOnce` false
    (:`Completed`
      (`UserWidget.AddToViewport` (`self.DeathScreen`) 0)
      (`WidgetBlueprintLibrary.SetInputMode_GameAndUIEx` (`GameplayStatics.GetPlayerController` 0) (`/Game/UI/DeathScreen.Resume_Btn` (stale `self.ReceiveBeginPlay` _returnvalue_3)) "DoNotLock" false))))

(fn `UserConstructionScript`)