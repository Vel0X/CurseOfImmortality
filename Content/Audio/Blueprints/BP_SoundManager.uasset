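; BP_SoundManager is a sound manager that plays game sounds by name.
; Three Impl events look the name up in SoundMap and, if found, play it as 2D, at a given location, or attached to a component.
; The graph also holds unconnected CustomGameMode getter nodes that never run, and the construction script is empty.
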(event `self.PlaySoundImpl`
  (params (Name :type String))
  (bind (_value _returnvalue) (`BlueprintMapLibrary.Map_Find` (`self.SoundMap`) Name))
  (if _returnvalue
    (`GameplayStatics.PlaySound2D` _value 1.0 1.0 0.0 null null)))

(event `self.PlaySoundLocatedImpl`
  (params (Position :type "Vector Structure (by ref)") (Name :type String))
  (bind (_value _returnvalue) (`BlueprintMapLibrary.Map_Find` (`self.SoundMap`) Name))
  (if _returnvalue
    (`GameplayStatics.PlaySoundAtLocation` _value Position (struct) 1.0 1.0 0.0 null null null null)))

(event `self.PlaySoundAttachedImpl`
  (params (Component :type "SceneComponent Object Reference") (Name :type String))
  (bind (_value _returnvalue) (`BlueprintMapLibrary.Map_Find` (`self.SoundMap`) Name))
  (if _returnvalue
    (`GameplayStatics.SpawnSoundAttached` _value Component "None" (0.0 0.0 0.0) (struct) "KeepRelativeOffset" false 1.0 1.0 0.0 null null)))

(fn `UserConstructionScript`)