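; Small right-hand gate actor that animates three brace components toward their open "Up" positions as soon as play begins.
; Tick calls GateUp, sliding Brace and Brace3 in opposite directions along relative X and raising Brace6 along Z.
; Movement scales with Speed and delta time, each axis stopping once it passes its stored limit, without clamping.
; GateDown mirrors this toward the base positions but is never executed.
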(event `self.ReceiveTick`
  (params (DeltaSeconds :type "Float (single-precision)"))
  (`self.GateUp` DeltaSeconds))

(fn `GateDown`
  (params (DeltaTime :type "Float (double-precision)"))
  (bind (_posbrace6_x _posbrace6_y _posbrace6_z) (`KismetMathLibrary.BreakVector` (`self.posBrace6`)))
  (bind _brace6 (`self.Brace6`))
  (bind _posbrace_x (`KismetMathLibrary.BreakVector` (`self.posBrace`)))
  (bind _brace3 (`self.Brace3`))
  (bind _posbrace3_x (`KismetMathLibrary.BreakVector` (`self.posBrace3`)))
  (bind _returnvalue (`SceneComponent.GetRelativeTransform` (`self.Brace`)))
  (bind _returnvalue_2 (`SceneComponent.GetRelativeTransform` _brace3))
  (bind _returnvalue_3 (`SceneComponent.GetRelativeTransform` _brace6))
  (`|ExecutionSequence`
    (:`then_0`
      (if (not (<= (.x (.location _returnvalue)) _posbrace_x))
        (`SceneComponent.K2_SetRelativeLocation` (`self.Brace`) (`KismetMathLibrary.MakeVector` (- (.x (.location _returnvalue)) (* DeltaTime (`self.Speed`))) (.y (.location _returnvalue)) (.z (.location _returnvalue))) false false)))
    (:`then_1`
      (if (not (>= (.x (.location _returnvalue_2)) _posbrace3_x))
        (`SceneComponent.K2_SetRelativeLocation` _brace3 (`KismetMathLibrary.MakeVector` (+ (.x (.location _returnvalue_2)) (* DeltaTime (`self.Speed`))) (.y (.location _returnvalue_2)) (.z (.location _returnvalue_2))) false false)))
    (:`then_2`
      (if (not (<= (.z (.location _returnvalue_3)) _posbrace6_z))
        (`SceneComponent.K2_SetRelativeLocation` _brace6 (`KismetMathLibrary.MakeVector` (.x (.location _returnvalue_3)) (.y (.location _returnvalue_3)) (- (.z (.location _returnvalue_3)) (* DeltaTime (`self.Speed`)))) false false)))))

(fn `GateUp`
  (params (DeltaTime :type "Float (double-precision)"))
  (bind _brace6 (`self.Brace6`))
  (bind _posbraceup_x (`KismetMathLibrary.BreakVector` (`self.posBraceUp`)))
  (bind _posbrace3up_x (`KismetMathLibrary.BreakVector` (`self.posBrace3Up`)))
  (bind (_posbrace6up_x _posbrace6up_y _posbrace6up_z) (`KismetMathLibrary.BreakVector` (`self.posBrace6Up`)))
  (bind _brace3 (`self.Brace3`))
  (bind _returnvalue (`SceneComponent.GetRelativeTransform` (`self.Brace`)))
  (bind _returnvalue_2 (`SceneComponent.GetRelativeTransform` _brace3))
  (bind _returnvalue_3 (`SceneComponent.GetRelativeTransform` _brace6))
  (`|ExecutionSequence`
    (:`then_0`
      (if (not (>= (.x (.location _returnvalue)) _posbraceup_x))
        (`SceneComponent.K2_SetRelativeLocation` (`self.Brace`) (`KismetMathLibrary.MakeVector` (+ (.x (.location _returnvalue)) (* DeltaTime (`self.Speed`))) (.y (.location _returnvalue)) (.z (.location _returnvalue))) false false)))
    (:`then_1`
      (if (not (<= (.x (.location _returnvalue_2)) _posbrace3up_x))
        (`SceneComponent.K2_SetRelativeLocation` _brace3 (`KismetMathLibrary.MakeVector` (- (.x (.location _returnvalue_2)) (* DeltaTime (`self.Speed`))) (.y (.location _returnvalue_2)) (.z (.location _returnvalue_2))) false false)))
    (:`then_2`
      (if (not (>= (.z (.location _returnvalue_3)) _posbrace6up_z))
        (`SceneComponent.K2_SetRelativeLocation` _brace6 (`KismetMathLibrary.MakeVector` (.x (.location _returnvalue_3)) (.y (.location _returnvalue_3)) (+ (.z (.location _returnvalue_3)) (* DeltaTime (`self.Speed`)))) false false)))))

(fn `UserConstructionScript`)