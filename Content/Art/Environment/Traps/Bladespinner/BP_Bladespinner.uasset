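; Bladespinner environment trap with a spinning blade mesh and a knife hitbox tied to a damage component.
; Tick spins the cylinder around yaw by Speed and mirrors the Trap's active flag onto its visibility and overlap events.
; Ending an overlap on the knife collider resets that hitbox's hit-character list.
; DisableTrap deactivates the trap, turns off its collision and hides the whole actor.
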(event `self.ReceiveTick`
  (params (DeltaSeconds :type "Float (single-precision)"))
  (bind (_returnvalue_roll _returnvalue_pitch _returnvalue_yaw) (`KismetMathLibrary.BreakRotator` (`SceneComponent.K2_GetComponentRotation` (`self.Bladespinner_Cylinder_002`))))
  (`self.SetVisibility`)
  (`SceneComponent.K2_SetWorldRotation` (`self.Bladespinner_Cylinder_002`) (`KismetMathLibrary.MakeRotator` _returnvalue_roll _returnvalue_pitch (- _returnvalue_yaw (* DeltaSeconds (`self.Speed`)))) false false))

(event `self.knifecol.OnComponentEndOverlap`
  (params (OverlappedComponent :type "PrimitiveComponent Object Reference") (OtherActor :type "Actor Object Reference") (OtherComp :type "PrimitiveComponent Object Reference") (OtherBodyIndex :type Integer))
  (`DamageComponent.ResetHitCharactersForHitbox` (`self.DamageComponent`) (`self.knifecol`)))

(event `self.DisableTrap`
  (set `TrapComponent.TrapIsActive` false (`self.Trap`))
  (`PrimitiveComponent.SetCollisionEnabled` (`self.TrapCollision`) "NoCollision")
  (`PrimitiveComponent.SetCollisionEnabled` (`self.Capsule`) "NoCollision")
  (`PrimitiveComponent.SetCollisionEnabled` (`self.knifecol`) "NoCollision")
  (`SceneComponent.SetVisibility` (`self.DefaultSceneRoot`) false true))

(fn `SetVisibility`
  (bind _knifecol (`self.knifecol`))
  (bind _trapcollision (`self.TrapCollision`))
  (bind _bladespinner_cylinder_002 (`self.Bladespinner_Cylinder_002`))
  (if (`TrapComponent.TrapIsActive` (`self.Trap`))
    (`SceneComponent.SetVisibility` _bladespinner_cylinder_002 true true)
    (set `PrimitiveComponent.bGenerateOverlapEvents` true _trapcollision)
    (set `PrimitiveComponent.bGenerateOverlapEvents` true _knifecol)
    (else
      (`SceneComponent.SetVisibility` _bladespinner_cylinder_002 false true)
      (set `PrimitiveComponent.bGenerateOverlapEvents` false _trapcollision)
      (set `PrimitiveComponent.bGenerateOverlapEvents` false _knifecol))))

(fn `UserConstructionScript`)