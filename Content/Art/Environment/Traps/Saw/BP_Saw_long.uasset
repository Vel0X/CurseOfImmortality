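; BP_Saw_long is a saw blade trap that spins its blade and shuttles its collision back and forth along a track.
; Each Tick rotates the blade and steps SawCollision along the normalized target vector at fixed height, swapping between two local endpoints on arrival.
; Tick also syncs mesh visibility and overlap events to TrapComponent.TrapIsActive.
; DisableTrap clears that flag, turns off collision and hides the root.
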(event `self.ReceiveBeginPlay`)

(event `self.ReceiveTick`
  (params (DeltaSeconds :type "Float (single-precision)"))
  (bind _newvar_0 (`self.NewVar_0`))
  (bind _newvar_1 (`self.NewVar_1`))
  (bind _returnvalue_location (`KismetMathLibrary.BreakTransform` (`SceneComponent.GetRelativeTransform` (`self.SawCollision`))))
  (bind (_returnvalue_x _returnvalue_y) (`KismetMathLibrary.BreakVector` (+ (`KismetMathLibrary.Normal` _newvar_0) _returnvalue_location)))
  (`self.Set Visibility`)
  (`SceneComponent.K2_AddRelativeRotation` (`self.saw_SawBlade`) (struct :`Roll` 15.0) false false)
  (if (== _returnvalue_location _newvar_0 :`ErrorTolerance` 2.0)
    (if (== _newvar_0 _newvar_1)
      (set `self.NewVar_0` (`self.NewVar_2`))
      (else
        (set `self.NewVar_0` _newvar_1)))
    (else
      (`SceneComponent.K2_SetRelativeLocation` (`self.SawCollision`) (`KismetMathLibrary.MakeVector` _returnvalue_x _returnvalue_y 10.0) false false))))

(event `self.DisableTrap`
  (set `TrapComponent.TrapIsActive` false (`self.TrapComponent`))
  (`PrimitiveComponent.SetCollisionEnabled` (`self.Box`) "NoCollision")
  (`PrimitiveComponent.SetCollisionEnabled` (`self.SawCollision`) "NoCollision")
  (`SceneComponent.SetVisibility` (`self.Root`) false false))

(fn `Set Visibility`
  (bind _saw_sawsocket (`self.saw_SawSocket`))
  (bind _sawcollision (`self.SawCollision`))
  (bind _sawcollision_2 (`self.SawCollision`))
  (if (`TrapComponent.TrapIsActive` (`self.TrapComponent`))
    (`SceneComponent.SetVisibility` _saw_sawsocket true false)
    (`SceneComponent.SetVisibility` (`self.saw_SawBlade`) true false)
    (set `PrimitiveComponent.bGenerateOverlapEvents` true _sawcollision_2)
    (set `PrimitiveComponent.bGenerateOverlapEvents` true _sawcollision)
    (else
      (`SceneComponent.SetVisibility` _saw_sawsocket false false)
      (`SceneComponent.SetVisibility` (`self.saw_SawBlade`) false false)
      (set `PrimitiveComponent.bGenerateOverlapEvents` false _sawcollision_2)
      (set `PrimitiveComponent.bGenerateOverlapEvents` false _sawcollision))))

(fn `UserConstructionScript`)