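; BP_Saw_short is a saw trap with a spinning blade that shuttles between two relative positions.
; Each Tick spins the blade and steps SawCollision one unit along the normalized target vector, swapping targets within tolerance, so motion is frame-rate dependent.
; SetVisibility also runs each Tick, matching blade and socket visibility and both collisions' overlap events to TrapComponent.TrapIsActive.
; An older offset-and-speed movement path remains disconnected.
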(event `self.ReceiveBeginPlay`)

(event `self.ReceiveTick`
  (params (DeltaSeconds :type "Float (single-precision)"))
  (bind _newvar_0 (`self.NewVar_0`))
  (bind _newvar_1 (`self.NewVar_1`))
  (bind _returnvalue_location (`KismetMathLibrary.BreakTransform` (`SceneComponent.GetRelativeTransform` (`self.SawCollision`))))
  (set `self.Delta Seconds` DeltaSeconds)
  (`self.SetVisibility`)
  (`SceneComponent.K2_AddRelativeRotation` (`self.saw_SawBlade`) (struct :`Roll` 15.0) false false)
  (if (== _returnvalue_location _newvar_0 :`ErrorTolerance` 2.0)
    (if (== _newvar_0 _newvar_1)
      (set `self.NewVar_0` (`self.NewVar_2`))
      (else
        (set `self.NewVar_0` _newvar_1)))
    (else
      (`SceneComponent.K2_SetRelativeLocation` (`self.SawCollision`) (+ (`KismetMathLibrary.Normal` _newvar_0) _returnvalue_location) false false))))

(fn `CalculateCurrentOffset`
  (bind (_startlocation_x _startlocation_y) (`KismetMathLibrary.BreakVector` (`self.StartLocation`)))
  (bind (_relativelocation_x _relativelocation_y) (`KismetMathLibrary.BreakVector` (`SceneComponent.RelativeLocation` (`self.SawCollision`))))
  (set `self.CurrentOffset` (`KismetMathLibrary.Abs` (- _relativelocation_y _startlocation_y))))

(fn `MoveInDirection`
  (`SceneComponent.K2_SetWorldLocation` (`self.SawCollision`) (+ (* (`SceneComponent.GetRightVector` (`self.SawCollision`)) (`self.Delta Seconds`) (`self.Speed`)) (`SceneComponent.K2_GetComponentLocation` (`self.SawCollision`))) false false))

(fn `SetVisibility`
  (bind _saw_sawsocket (`self.saw_SawSocket`))
  (bind _trapcollision (`self.TrapCollision`))
  (bind _sawcollision (`self.SawCollision`))
  (if (`TrapComponent.TrapIsActive` (`self.TrapComponent`))
    (`SceneComponent.SetVisibility` _saw_sawsocket true false)
    (`SceneComponent.SetVisibility` (`self.saw_SawBlade`) true false)
    (set `PrimitiveComponent.bGenerateOverlapEvents` true _trapcollision)
    (set `PrimitiveComponent.bGenerateOverlapEvents` true _sawcollision)
    (else
      (`SceneComponent.SetVisibility` _saw_sawsocket false false)
      (`SceneComponent.SetVisibility` (`self.saw_SawBlade`) false false)
      (set `PrimitiveComponent.bGenerateOverlapEvents` false _trapcollision)
      (set `PrimitiveComponent.bGenerateOverlapEvents` false _sawcollision))))

(fn `UserConstructionScript`)