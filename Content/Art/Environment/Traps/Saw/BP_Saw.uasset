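; BP_Saw is an environment trap Blueprint that moves its SawCylinder component, apparently back and forth between two relative positions.
; Each Tick steps the saw one unit along the normalized target vector NewVar0, not the offset toward it, so speed depends on frame rate.
; When the saw is within tolerance of NewVar0, the target switches between NewVar1 and NewVar2.
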(event `self.ReceiveBeginPlay`)

(event `self.ReceiveTick`
  (params (DeltaSeconds :type "Float (single-precision)"))
  (bind _newvar_0 (`self.NewVar_0`))
  (bind _newvar_1 (`self.NewVar_1`))
  (bind _returnvalue_location (`KismetMathLibrary.BreakTransform` (`SceneComponent.GetRelativeTransform` (`self.saw_Cylinder`))))
  (if (== _returnvalue_location _newvar_0 :`ErrorTolerance` 2.0)
    (if (== _newvar_0 _newvar_1)
      (set `self.NewVar_0` (`self.NewVar_2`))
      (else
        (set `self.NewVar_0` _newvar_1)))
    (else
      (`SceneComponent.K2_SetRelativeLocation` (`self.saw_Cylinder`) (+ (`KismetMathLibrary.Normal` _newvar_0) _returnvalue_location) false false))))

(fn `UserConstructionScript`)